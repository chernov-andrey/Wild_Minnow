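; BP_Test is a player controller that lets the player trigger the next move of nearby AI characters.
; On BeginPlay it adds the default Enhanced Input mapping context to its local player subsystem.
; When the Actions input starts, it checks BP_AI_Base actors overlapping the controlled pawn and calls NextMove on each one flagged as having the player in range.
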(event `self.ReceiveBeginPlay`
  (bind _returnvalue (pcsubsystem `EnhancedInputLocalPlayerSubsystem` self))
  (`/Engine/EditorBlueprintResources/StandardMacros.IsValid` _returnvalue
    (:`Is Valid`
      (`EnhancedInputSubsystemInterface.AddMappingContext` _returnvalue "/Game/GameSettings/Input/IMC_Default.IMC_Default" 0 (struct)))))

(event `EnhancedInput|/Game/GameSettings/Input/Actions/IA_Actions`
  (params (ActionValue :type Boolean) (ElapsedSeconds :type "Float (double-precision)") (TriggeredSeconds :type "Float (double-precision)") (InputAction :type "InputAction Object Reference" :default "/Game/GameSettings/Input/Actions/IA_Actions.IA_Actions"))
  (:`Started`
    (for _array_element (`self.GetOverlappingActors` (`self.K2_GetPawn`) "/Game/Blueprints/Character/BP_AI_Base.BP_AI_Base_C")
      (bind _asbp_ai_base (cast `/Game/Blueprints/Character/BP_AI_Base` _array_element))
      (if (`/Game/Blueprints/Character/BP_AI_Base.PlayerInRange` _asbp_ai_base)
        (`/Game/Blueprints/Character/BP_AI_Base.NextMove` _asbp_ai_base)))))

(fn `UserConstructionScript`)