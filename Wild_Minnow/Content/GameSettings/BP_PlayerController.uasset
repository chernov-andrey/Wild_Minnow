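; Player controller that sets up input, camera and music playback for the game.
; On BeginPlay it adds the default Enhanced Input mapping context, and on possess it switches the view target to the level's BP_CameraPawn.
; Hotkeys open the scores screen widget and, as a debug key, the pause menu through the game instance.
; PlayMusic and StopMusic drive a single Audio component.
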(event EventBeginPlay
  (bind _self self)
  (bind _returnvalue (PlayerController|LocalPlayerSubsystems|GetEnhancedInputLocalPlayerSubsystem _self))
  (Utilities|IsValid _returnvalue
    (:Is%20Valid
      (Input|AddMappingContext _returnvalue "/Game/GameSettings/Input/IMC_Default.IMC_Default" 0 "(bIgnoreAllPressedKeysUntilRelease=True,bForceImmediately=False,bNotifyUserSettings=False)"))))

(event EventStopMusic
  (Audio|Components|Audio|Stop (Variables|Default|GetAudio)))

(event EventPossess
  (params (PossessedPawn :type Pawn%20Object%20Reference))
  (bind _returnvalue (Actor|GetActorOfClass "/Game/GameSettings/BP_CameraPawn.BP_CameraPawn_C"))
  (Game|Player|SetViewTargetwithBlend _returnvalue 0.0 "VTBlend_Linear" 0.0 false))

(event Input|KeyboardEvents|DebugKeyP
  (params (Key :type Key%20Structure :default "None") (ActionValue :type Input%20Action%20Value%20Structure))
  (:Pressed
    (bind _asbp_game_instance_wm (Utilities|Casting|CastToBP_GameInstance_WM (Game|GetGameInstance)))
    (Class|GameInstanceWM|OpenPauseMenu _asbp_game_instance_wm)))

(event Input|KeyboardEvents|K
  (params (Key :type Key%20Structure :default "None"))
  (:Pressed
    (bind _returnvalue (UserInterface|CreateWidget "/Game/GUI/WBP_ScoresScreen.WBP_ScoresScreen_C"))
    (UserInterface|Viewport|AddtoViewport _returnvalue 0)))

(fn ConstructionScript)

(fn PlayMusic
  (params (Sound :type Sound%20Base%20Object%20Reference))
  (bind _audio (Variables|Default|GetAudio))
  (Audio|Components|Audio|SetSound _audio Sound)
  (Audio|Components|Audio|Play _audio 0.0)
  (return))