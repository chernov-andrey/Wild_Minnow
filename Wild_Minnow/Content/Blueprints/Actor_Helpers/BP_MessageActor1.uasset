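; BP_MessageActor1 is an actor that shows an on-screen info message while the player's pawn overlaps its Message component.
; On BeginPlay it creates a BPW_InfoMessage widget from WidgetClass, adds it hidden to the viewport, sets itself as owner and fills the text from ThisMessage.StringMessage.
; The component's begin and end overlap events toggle the widget's visibility, reacting only to player 0's pawn.
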(event `self.ReceiveBeginPlay`
  (bind _this_message_stringmessage (break `/Game/Blueprints/Actor_Helpers/ST_Messages` (`self.This Message`)))
  ;[1 1 1] Инициализация виджета
  (bind _returnvalue (`|CreateWidget` (`self.WidgetClass`)))
  (bind _asbpw_info_message (cast `/Game/GUI/BPW_InfoMessage` _returnvalue))
  (bind _output_get (set `self.Widget Message` _asbpw_info_message))
  (`Widget.SetVisibility` _output_get "Hidden")
  (`UserWidget.AddToViewport` (`self.Widget Message`) 0)
  (`/Game/GUI/BPW_InfoMessage.Set Owner` (`self.Widget Message`) self)
  (`/Game/GUI/BPW_InfoMessage.Set Text` (`self.Widget Message`) _this_message_stringmessage)
  (`/Game/GUI/BPW_InfoMessage.Set Text` (`self.Widget Message`) _this_message_stringmessage))

(event `self.Message.OnComponentBeginOverlap`
  (params (OverlappedComponent :type "PrimitiveComponent Object Reference") (OtherActor :type "Actor Object Reference") (OtherComp :type "PrimitiveComponent Object Reference") (OtherBodyIndex :type Integer) (bFromSweep :type Boolean) (SweepResult :type "HitResult Structure (by ref)"))
  ;[1 1 1] Когда объект посещает оверлап, сделать объект видимым
  (if (== OtherActor (`GameplayStatics.GetPlayerPawn` 0))
    (`Widget.SetVisibility` (`self.Widget Message`) "Visible")))

(event `self.Message.OnComponentEndOverlap`
  (params (OverlappedComponent :type "PrimitiveComponent Object Reference") (OtherActor :type "Actor Object Reference") (OtherComp :type "PrimitiveComponent Object Reference") (OtherBodyIndex :type Integer))
  ;[1 1 1] Когда объект покидает оверлап, сделать виджет невидимым
  (if (== OtherActor (`GameplayStatics.GetPlayerPawn` 0))
    (`Widget.SetVisibility` (`self.Widget Message`) "Hidden")))

(fn `UserConstructionScript`)