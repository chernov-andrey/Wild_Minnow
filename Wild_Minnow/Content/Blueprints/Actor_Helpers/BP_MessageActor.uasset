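; BP_MessageActor is a helper actor that shows a button prompt widget while the player is near it.
; On BeginPlay it creates a BPW_Button widget, adds it to the viewport hidden and keeps a reference.
; Overlap begin and end events on its Message component show and hide that widget, reacting only to the first player's pawn.
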(event `self.ReceiveBeginPlay`
  (bind _returnvalue (`|CreateWidget` "/Game/GUI/BPW_Button.BPW_Button_C"))
  (bind _output_get (set `self.Widget Button` _returnvalue))
  (`Widget.SetVisibility` _output_get "Hidden")
  (`UserWidget.AddToViewport` (`self.Widget Button`) 0))

(event `self.Message.OnComponentBeginOverlap`
  (params (OverlappedComponent :type "PrimitiveComponent Object Reference") (OtherActor :type "Actor Object Reference") (OtherComp :type "PrimitiveComponent Object Reference") (OtherBodyIndex :type Integer) (bFromSweep :type Boolean) (SweepResult :type "HitResult Structure (by ref)"))
  (if (== OtherActor (`GameplayStatics.GetPlayerPawn` 0))
    (`Widget.SetVisibility` (`self.Widget Button`) "Visible")))

(event `self.Message.OnComponentEndOverlap`
  (params (OverlappedComponent :type "PrimitiveComponent Object Reference") (OtherActor :type "Actor Object Reference") (OtherComp :type "PrimitiveComponent Object Reference") (OtherBodyIndex :type Integer))
  (if (== OtherActor (`GameplayStatics.GetPlayerPawn` 0))
    (`Widget.SetVisibility` (`self.Widget Button`) "Hidden")))

(fn `UserConstructionScript`)