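; Base environment object that hands a resource to the player when clicked.
; On BeginPlay it sets its flipbook's world roll from the camera pawn spring arm's pitch, a one-time tilt toward the camera.
; A sprite click checks for the player character inside CollectResourcesBox, then passes it the resource message from CBPResources.
; The actor's own resource functions are stubs returning default values.
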(event `self.ReceiveBeginPlay`
  ;[1 1 1] Ориентация объекта по направлению к камере
  (bind _returnvalue (`GameplayStatics.GetActorOfClass` "/Game/GameSettings/BP_CameraPawn.BP_CameraPawn_C"))
  (bind (_returnvalue_roll _returnvalue_pitch) (`KismetMathLibrary.BreakRotator` (`SpringArmComponent.GetTargetRotation` (`/Game/GameSettings/BP_CameraPawn.SpringArm` _returnvalue))))
  (`SceneComponent.K2_SetWorldRotation` (`self.PaperFlipbook`) (`KismetMathLibrary.MakeRotator` _returnvalue_pitch) false false))

(event `self.PaperSprite.OnClicked`
  (params (TouchedComponent :type "PrimitiveComponent Object Reference") (ButtonPressed :type "Key Structure"))
  ;[1 1 1] Если по объекту тыкнули мышкой, проверяем, близко ли персонаж игрока, если близко, то передаём ему наш ресурс
  (for _array_element (`PrimitiveComponent.GetOverlappingActors` (`self.Collect Resources Box`) "/Game/Blueprints/Character/Character/BP_Character.BP_Character_C")
    (set `self.Array Element` _array_element)
    (if (== _array_element (`GameplayStatics.GetPlayerCharacter` 0))
      (bind _type_of_resource (`/Game/Blueprints/Components/CBP_Resources.Get Type of Resource` (`self.CBP_Resources`)))
      (bind (_type_of_resource_out _counter) (message `/Game/Blueprints/Interfaces/IBP_Resources.Get Resource` (`self.CBP_Resources`) _type_of_resource))
      (message `/Game/Blueprints/Interfaces/IBP_Resources.Give Resource` (`self.Array Element`) _type_of_resource_out _counter))))

(fn `Decrease Resource`
  (params (`Type of Resource` :type "/Game/Blueprints/Enviroment/Enum_Resources Enum" :default "NewEnumerator0") (Value :type "Float (double-precision)"))
  (returns (Success :type Boolean))
  (return false))

(fn `Get Resource`
  (params (`Type of Resource in` :type "/Game/Blueprints/Enviroment/Enum_Resources Enum" :default "NewEnumerator0"))
  (returns (`Type of Resource out` :type "/Game/Blueprints/Enviroment/Enum_Resources Enum") (Counter :type "Float (double-precision)"))
  (return "NewEnumerator0" 0.0))

(fn `Get Type of Resorce`
  (returns (NewParam :type "/Game/Blueprints/Enviroment/Enum_Resources Enum"))
  (return "NewEnumerator0"))

(fn `UserConstructionScript`)