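; Campfire actor that lights when something enters its interaction sphere and returns to its unlit look when the overlap ends.
; ApplyFireState switches the Paper2D flipbook, looping and Niagara effect visibility for three states: Unit (unlit), Igniting and Always.
; Overlap begin plays the one-shot ignition, then after a short delay switches to the looping full fire.
; A separate TryIgnite event triggers ignition only if the Firestate variable is Unit.
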(event `TryIgnite`
  (if (`|EnumEquality` (`self.Firestate`) "NewEnumerator0")
    (`self.ApplyFireState` "NewEnumerator1")))

(event `self.ReceiveBeginPlay`
  (`parent.ReceiveBeginPlay`)
  (`self.ApplyFireState` "NewEnumerator0"))

(event `self.InteractSphere.OnComponentBeginOverlap`
  (params (OverlappedComponent :type "PrimitiveComponent Object Reference") (OtherActor :type "Actor Object Reference") (OtherComp :type "PrimitiveComponent Object Reference") (OtherBodyIndex :type Integer) (bFromSweep :type Boolean) (SweepResult :type "HitResult Structure (by ref)"))
  (`self.ApplyFireState` "NewEnumerator1")
  (`KismetSystemLibrary.Delay` 0.25)
  (`self.ApplyFireState` "NewEnumerator2"))

(event `self.InteractSphere.OnComponentEndOverlap`
  (params (OverlappedComponent :type "PrimitiveComponent Object Reference") (OtherActor :type "Actor Object Reference") (OtherComp :type "PrimitiveComponent Object Reference") (OtherBodyIndex :type Integer))
  (`self.ApplyFireState` "NewEnumerator0"))

(fn `ApplyFireState`
  (params (Firestate :type "/Game/Blueprints/Enviroment/CampFire/Enum_FireState Enum" :default "NewEnumerator0"))
  (switch `/Game/Blueprints/Enviroment/CampFire/Enum_FireState` Firestate
    (:`NewEnumerator0`
      (`PaperFlipbookComponent.SetFlipbook` (`self.PaperFlipbook`) "/Game/Art/PaperAssets/Enviroment/Firecamp/Nofire/Firecamp.Firecamp")
      (`PaperFlipbookComponent.SetLooping` (`self.PaperFlipbook`) false)
      (`SceneComponent.SetVisibility` (`self.Niagara`) false false))
    (:`NewEnumerator1`
      (`PaperFlipbookComponent.SetFlipbook` (`self.PaperFlipbook`) "/Game/Art/PaperAssets/Enviroment/Firecamp/Ignition/Firecamp1.Firecamp1")
      (`PaperFlipbookComponent.SetLooping` (`self.PaperFlipbook`) false)
      (`PaperFlipbookComponent.PlayFromStart` (`self.PaperFlipbook`))
      (`SceneComponent.SetVisibility` (`self.Niagara`) true false))
    (:`NewEnumerator2`
      (`PaperFlipbookComponent.SetFlipbook` (`self.PaperFlipbook`) "/Game/Art/PaperAssets/Enviroment/Firecamp/Always/Firecampfull1.Firecampfull1")
      (`PaperFlipbookComponent.SetLooping` (`self.PaperFlipbook`) true)
      (`PaperFlipbookComponent.PlayFromStart` (`self.PaperFlipbook`))
      (`SceneComponent.SetVisibility` (`self.Niagara`) true false))))

(fn `UserConstructionScript`
  (`parent.UserConstructionScript`))