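; BP_Redberry is an environment berry plant that animates berries growing when something overlaps its interact sphere.
; ApllyBerryState swaps the Paper2D flipbook between Noberry, Growth and Fullberry as non-looping animations, restarting playback for the latter two.
; It starts at Noberry; overlap plays Growth, then Fullberry after a short delay.
; Ending overlap resets to Noberry but leaves any pending delay running, so Fullberry can still appear afterward.
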(event `self.ReceiveBeginPlay`
  (`parent.ReceiveBeginPlay`)
  (`self.ApllyBerryState` "NewEnumerator0"))

(event `self.InteractSphere.OnComponentBeginOverlap`
  (params (OverlappedComponent :type "PrimitiveComponent Object Reference") (OtherActor :type "Actor Object Reference") (OtherComp :type "PrimitiveComponent Object Reference") (OtherBodyIndex :type Integer) (bFromSweep :type Boolean) (SweepResult :type "HitResult Structure (by ref)"))
  (`self.ApllyBerryState` "NewEnumerator1")
  (`KismetSystemLibrary.Delay` 1.0)
  (`self.ApllyBerryState` "NewEnumerator2"))

(event `self.InteractSphere.OnComponentEndOverlap`
  (params (OverlappedComponent :type "PrimitiveComponent Object Reference") (OtherActor :type "Actor Object Reference") (OtherComp :type "PrimitiveComponent Object Reference") (OtherBodyIndex :type Integer))
  (`self.ApllyBerryState` "NewEnumerator0"))

(fn `ApllyBerryState`
  (params (Selection :type "/Game/Blueprints/Enviroment/Blueberry/Enums_Blueberry Enum" :default "NewEnumerator0"))
  (switch `/Game/Blueprints/Enviroment/Blueberry/Enums_Blueberry` Selection
    (:`NewEnumerator0`
      (`PaperFlipbookComponent.SetFlipbook` (`self.PaperFlipbook`) "/Game/Art/PaperAssets/Enviroment/Rebberry/NoBerry/Noberry.Noberry")
      (`PaperFlipbookComponent.SetLooping` (`self.PaperFlipbook`) false))
    (:`NewEnumerator1`
      (`PaperFlipbookComponent.SetFlipbook` (`self.PaperFlipbook`) "/Game/Art/PaperAssets/Enviroment/Rebberry/Growth/Growth.Growth")
      (`PaperFlipbookComponent.SetLooping` (`self.PaperFlipbook`) false)
      (`PaperFlipbookComponent.PlayFromStart` (`self.PaperFlipbook`)))
    (:`NewEnumerator2`
      (`PaperFlipbookComponent.SetFlipbook` (`self.PaperFlipbook`) "/Game/Art/PaperAssets/Enviroment/Rebberry/FullBerry/Fullberry.Fullberry")
      (`PaperFlipbookComponent.SetLooping` (`self.PaperFlipbook`) false)
      (`PaperFlipbookComponent.PlayFromStart` (`self.PaperFlipbook`)))))

(fn `UserConstructionScript`
  (`parent.UserConstructionScript`))