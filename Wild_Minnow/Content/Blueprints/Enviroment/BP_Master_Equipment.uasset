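; Base actor for equipment containers: a Paper2D sprite tilted to the camera's spring arm that the player can pick up and carry.
; On click, if the player overlaps CollectResourcesBox and accepts it as a heavy item, it teleports to an offset, attaches and calls Pickup.
; Gameplay tags, initially Empty, track state, while ChangeSprite swaps empty and full sprites.
; Hover changes the cursor; resource transfer functions return placeholder defaults.
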(event `self.ReceiveBeginPlay`
  (bind (_returnvalue_x _returnvalue_y _returnvalue_z) (`KismetMathLibrary.BreakVector` (`self.K2_GetActorLocation` self)))
  ;[1 1 1] Ориентация спрайта навстречу камере
  (bind _returnvalue (`GameplayStatics.GetActorOfClass` "/Game/GameSettings/BP_CameraPawn.BP_CameraPawn_C"))
  (bind (_returnvalue_roll _returnvalue_pitch) (`KismetMathLibrary.BreakRotator` (`SpringArmComponent.GetTargetRotation` (`/Game/GameSettings/BP_CameraPawn.SpringArm` _returnvalue))))
  (`SceneComponent.K2_SetWorldRotation` (`self.PaperSprite`) (`KismetMathLibrary.MakeRotator` _returnvalue_pitch) false false)
  ;[1 1 1] Объявляем, что этот контейнер пустой
  (`BlueprintGameplayTagLibrary.AddGameplayTag` (`self.EmptyTags`) (struct :`TagName` "Inventory Tags.Empty"))
  ;[1 1 1] Возможно лишнее, но пока оставим
  (set `self.ZOffset` _returnvalue_z)
  ;[1 1 1] Подписываемся на клик
  (add `PrimitiveComponent.OnClicked` (`self.PaperSprite`) (delegate `On Clicked Master`))
  (add `self.OnBeginCursorOver` (delegate `OnBeginCursorOver_Event`))
  (add `self.OnEndCursorOver` (delegate `OnEndCursorOver_Event`)))

(event `OnBeginCursorOver_Event` :!signature `self.OnBeginCursorOver`
  (params (TouchedActor :type "Actor Object Reference"))
  (bind _asbp_player_controller (cast `/Game/GameSettings/BP_PlayerController` (`GameplayStatics.GetPlayerController` 0)))
  (`/Game/GameSettings/BP_PlayerController.ChangeCursor` _asbp_player_controller 1))

(event `OnEndCursorOver_Event` :!signature `self.OnEndCursorOver`
  (params (TouchedActor :type "Actor Object Reference"))
  (bind _asbp_player_controller (cast `/Game/GameSettings/BP_PlayerController` (`GameplayStatics.GetPlayerController` 0)))
  (`/Game/GameSettings/BP_PlayerController.ChangeCursor` _asbp_player_controller 0))

(event `Try_Pickup`
  (bind (_returnvalue_x _returnvalue_y _returnvalue_z) (`KismetMathLibrary.BreakVector` (`self.K2_GetActorLocation` (`self.Array Element`))))
  ;[1 1 1] Если по объекту тыкнули мышкой, проверяем, близко ли персонаж игрока, если близко, то передаём ему наш ресурс
  (bind _clicked_by_player (`self.Clicked by Player?` (`self.Collect Resources Box`) :!label _label))
  (if _clicked_by_player
    (bind _success (message `/Game/Blueprints/Interfaces/IBP_Inventory.Set Heavy Item` (`self.Array Element`) self))
    (if _success
      (`self.K2_SetActorLocation` (`KismetMathLibrary.MakeVector` _returnvalue_x (- _returnvalue_y 175.0) (+ _returnvalue_z 175.0)) false true)
      (bind _returnvalue (`self.K2_AttachToActor` (`self.Array Element`) "None" "KeepWorld" "KeepWorld" "KeepWorld" false))
      (set `self.This attached` _returnvalue)
      (`self.Pickup`)
      (else
        (`KismetSystemLibrary.PrintString` "Я уже несу вещь")))))

(event `On Clicked Master`
  (params (TouchedComponent :type "PrimitiveComponent Object Reference") (ButtonPressed :type "Key Structure" :default "None"))
  ;[1 1 1] Если по объекту тыкнули мышкой, проверяем, близко ли персонаж игрока, если близко, то передаём ему наш ресурс
  (goto _label))

(event `/Game/Blueprints/Interfaces/IBP_Inventory.Add Tag`
  (params (Tag :type "GameplayTag Structure"))
  (`BlueprintGameplayTagLibrary.AddGameplayTag` (`self.EmptyTags`) Tag))

(event `/Game/Blueprints/Interfaces/IBP_Inventory.Change Sprite`
  (params (`Inventory Tag` :type "GameplayTag Structure"))
  ;[1 1 1] Меняем спрайт в зависимости от того, пустой контейнер или нет
  (`|SwitchGameplayTag` `Inventory Tag`
    (:`Default`
      (`PaperSpriteComponent.SetSprite` (`self.PaperSprite`) (`self.Sprite Full`)))
    (:`Inventory Tags.Empty`
      (`PaperSpriteComponent.SetSprite` (`self.PaperSprite`) (`self.Sprite Empty`)))))

(event `/Game/Blueprints/Interfaces/IBP_Inventory.Remove Tag`
  (params (Tag :type "GameplayTag Structure"))
  (`BlueprintGameplayTagLibrary.RemoveGameplayTag` (`self.EmptyTags`) Tag))

(fn `Clicked by Player?`
  (params (`Box Collision` :type "BoxComponent Object Reference"))
  (returns (`Clicked by Player` :type Boolean))
  (for _array_element (`PrimitiveComponent.GetOverlappingActors` `Box Collision` "/Game/Blueprints/Character/Character/BP_Character.BP_Character_C")
    (set `self.Array Element` _array_element)
    (return (== _array_element (`GameplayStatics.GetPlayerCharacter` 0)))))

(fn `Decrease Resource`
  (params (`Type of Resource` :type "/Game/Blueprints/Enviroment/Enum_Resources Enum" :default "NewEnumerator0") (Value :type "Float (double-precision)"))
  (returns (Success :type Boolean))
  (return false))

(fn `Get Current Tag`
  (returns (`Current Tag` :type "GameplayTag Structure"))
  (return))

(fn `Get Inventory Gameplay Tag`
  (returns (`Inventory Tag` :type "GameplayTag Structure"))
  (return (`self.Inventory Tag`)))

(fn `Get Resource from this one`
  (params (`Type of Resource in` :type "/Game/Blueprints/Enviroment/Enum_Resources Enum" :default "NewEnumerator0"))
  (returns (`Type of Resource out` :type "/Game/Blueprints/Enviroment/Enum_Resources Enum") (Counter :type "Float (double-precision)") (Have :type Boolean))
  (return "NewEnumerator0" 0.0 false))

(fn `Get Type of Resorce`
  (returns (NewParam :type "/Game/Blueprints/Enviroment/Enum_Resources Enum"))
  (return "NewEnumerator0"))

(fn `Get ZOffset`
  (returns (`Get ZOffset` :type "Float (double-precision)"))
  (return (`self.ZOffset`)))

(fn `Give Resource to this one`
  (params (`Type of Resource` :type "/Game/Blueprints/Enviroment/Enum_Resources Enum" :default "NewEnumerator0") (Counter :type "Float (double-precision)"))
  (returns (`Have to Give` :type Boolean))
  (return false))

(fn `Has Tag`
  (params (Tag :type "GameplayTag Structure"))
  (returns (`Has Tag` :type Boolean))
  (return (`BlueprintGameplayTagLibrary.HasTag` (`self.EmptyTags`) Tag true)))

(fn `Remove T`
  (params (Tag :type "GameplayTag Structure"))
  (`BlueprintGameplayTagLibrary.RemoveGameplayTag` (`self.EmptyTags`) Tag))

(fn `Set Heavy Item`
  (params (Object :type "Actor Object Reference"))
  (returns (Success :type Boolean))
  (return false))

(fn `UserConstructionScript`)