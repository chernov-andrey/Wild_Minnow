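; BP_Well is a clickable well that gives the player a resource when they carry a bucket.
; It overrides the sprite's OnClicked without calling the parent, checking that the player character overlaps CollectResourcesBox and has the heavy-object Bucket inventory tag.
; It then gets the resource type and count from CBPResources and passes them to the character through GiveResourceMessage.
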(event `self.PaperSprite.OnClicked`
  (params (TouchedComponent :type "PrimitiveComponent Object Reference") (ButtonPressed :type "Key Structure"))
  ;[1 1 1] Переопределяю логику On Clicked, так как для неё нельзя вызвать родителя, логику нужно дополнить/изменить
  (for _array_element (`PrimitiveComponent.GetOverlappingActors` (`self.Collect Resources Box`) "/Game/Blueprints/Character/Character/BP_Character.BP_Character_C")
    (set `self.Array Element` _array_element)
    (if (== _array_element (`GameplayStatics.GetPlayerCharacter` 0))
      (bind _asbp_character (cast `/Game/Blueprints/Character/Character/BP_Character` (`self.Array Element`)))
      (bind _has_tag (`/Game/Blueprints/Character/Character/BP_Character.Has inventory Tag` _asbp_character (struct :`TagName` "Inventory Tags.Have Heavy Object.Bucket")))
      (if _has_tag
        (bind (_type_of_resource_out _counter) (message `/Game/Blueprints/Interfaces/IBP_Resources.Get Resource` (`self.CBP_Resources`) "NewEnumerator0"))
        (message `/Game/Blueprints/Interfaces/IBP_Resources.Give Resource` (`self.Array Element`) _type_of_resource_out _counter)))))

(fn `UserConstructionScript`
  (`parent.UserConstructionScript`))