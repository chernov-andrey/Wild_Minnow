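; Sawhorse prop that runs a sawing minigame through a SAW widget component when the player character is nearby.
; Sphere overlap shows the widget unless its last spawned Wood still exists; leaving resets and hides it.
; On completion it spawns a BP_Equip_UPDATE item beside itself as Wood, then resets and hides the widget after a short delay.
; Hovering over the widget switches the player controller's cursor.
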(event `self.ReceiveBeginPlay`
  (`parent.ReceiveBeginPlay`)
  (bind _assaw (cast `/Game/Test/MiniGame_saw/SAW` (`WidgetComponent.GetWidget` (`self.Saw_Game`))))
  (set `self.As SAW` _assaw))

(event `self.Sphere.OnComponentBeginOverlap`
  (params (OverlappedComponent :type "PrimitiveComponent Object Reference") (OtherActor :type "Actor Object Reference") (OtherComp :type "PrimitiveComponent Object Reference") (OtherBodyIndex :type Integer) (bFromSweep :type Boolean) (SweepResult :type "HitResult Structure (by ref)"))
  (bind _asbp_character_update (cast `/Game/Blueprints/Character/Character/BP_Character_UPDATE` OtherActor))
  (set `self.As BP Character` _asbp_character_update)
  (`/Engine/EditorBlueprintResources/StandardMacros.IsValid` (`self.Wood`)
    (:`Is Not Valid`
      (add `/Game/Test/MiniGame_saw/SAW.Complete_saw_game` (`self.As SAW`) (delegate `Complete`))
      (`SceneComponent.SetVisibility` (`self.Saw_Game`) true false))))

(event `self.Sphere.OnComponentEndOverlap`
  (params (OverlappedComponent :type "PrimitiveComponent Object Reference") (OtherActor :type "Actor Object Reference") (OtherComp :type "PrimitiveComponent Object Reference") (OtherBodyIndex :type Integer))
  (bind _asbp_character_update (cast `/Game/Blueprints/Character/Character/BP_Character_UPDATE` OtherActor))
  (if (== _asbp_character_update (`self.As BP Character`))
    (set `self.As BP Character` null)
    (`/Game/Test/MiniGame_saw/SAW.Reset_Widget` (`self.As SAW`))
    (`SceneComponent.SetVisibility` (`self.Saw_Game`) false false)))

(event `Complete`
  (bind (_returnvalue_x _returnvalue_y) (`KismetMathLibrary.BreakVector` (`self.K2_GetActorLocation` self)))
  (bind _returnvalue (`|SpawnActorFromClass` "/Game/Test/BP_Equip_UPDATE.BP_Equip_UPDATE_C" (`KismetMathLibrary.MakeTransform` (`KismetMathLibrary.MakeVector` (+ _returnvalue_x -100.0) (+ _returnvalue_y 100.0) 60.0) (struct) (0.04 0.04 0.04)) "Undefined" "MultiplyWithRoot" self false 0 "NewEnumerator1" null))
  (`SceneComponent.K2_SetWorldRotation` (`/Game/Test/BP_Equip_UPDATE.PaperSprite` _returnvalue) (struct :`Roll` -45.0) false false)
  (set `self.Wood` _returnvalue)
  (`KismetSystemLibrary.Delay` 1.0)
  (`/Game/Test/MiniGame_saw/SAW.Reset_Widget` (`self.As SAW`))
  (`SceneComponent.SetVisibility` (`self.Saw_Game`) false false))

(event `self.Saw_Game.OnBeginCursorOver`
  (params (TouchedComponent :type "PrimitiveComponent Object Reference"))
  (bind _asbp_player_controller (cast `/Game/GameSettings/BP_PlayerController` (`GameplayStatics.GetPlayerController` 0)))
  (`/Game/GameSettings/BP_PlayerController.ChangeCursor` _asbp_player_controller 1))

(event `self.Saw_Game.OnEndCursorOver`
  (params (TouchedComponent :type "PrimitiveComponent Object Reference"))
  (bind _asbp_player_controller (cast `/Game/GameSettings/BP_PlayerController` (`GameplayStatics.GetPlayerController` 0)))
  (`/Game/GameSettings/BP_PlayerController.ChangeCursor` _asbp_player_controller 0))

(fn `UserConstructionScript`
  (`parent.UserConstructionScript`))