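; Cauldron actor for brewing kisel, storing water, wood and blueberries in an inventory component and steadily burning wood each tick to drive the fire.
; Clicking it while the player is in range maps their carried-item gameplay tag to a resource and pulls it in via interface messages.
; Deposits update the state and fill widgets and recolor the kisel by berry-to-water ratio.
; InteractBox overlap toggles the operations and state widgets.
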(event `self.ReceiveBeginPlay`
  ;[1 1 1] Инициализацией
  (bind _asbpw_cauldron_operations (cast `/Game/GUI/BPW_CauldronOperations` (`WidgetComponent.GetWidget` (`self.Widget Operations with Cauldron`))))
  (set `self.As BPW Cauldron Operations` _asbpw_cauldron_operations)
  ;[1 1 1] Делаем виджет невидимым
  (`Widget.SetVisibility` (`self.As BPW Cauldron Operations`) "Hidden")
  ;[1 1 1] Инициализация виджета
  (bind _returnvalue (`|CreateWidget` "/Game/GUI/BPW_CauldronState.BPW_CauldronState_C"))
  (set `self.As BPW Cauldron State` _returnvalue)
  (`Widget.SetVisibility` (`self.As BPW Cauldron State`) "Hidden")
  (`UserWidget.AddToViewport` (`self.As BPW Cauldron State`) 0)
  (for _array_element (`self.EnumParam`)
    (`self.Update Widget` _array_element)
    ;[1 1 1] Сохраняем ссылку на виджет котла с прогресс баром
    (bind _asbpw_cauldron_widget (cast `/Game/GUI/BPW_Cauldron_Widget` (`WidgetComponent.GetWidget` (`self.Widget Cauldron`))))
    (set `self.As BPW Cauldron Widget` _asbpw_cauldron_widget)))

(event `self.ReceiveTick`
  (params (DeltaSeconds :type "Float (single-precision)"))
  ;[1 1 1] Постепенный и постоянный расход топлива
  (for _array_element (`self.EnumParam`)
    (bind _value_to_give (`/Game/Blueprints/Components/CBP_Inventory.Get Value of Resource` (`self.CBP_Inventory`) _array_element))
    (`KismetSystemLibrary.PrintString` (`KismetStringLibrary.Concat_StrStr` (`|GetEnumeratorNameAsString` _array_element) " " (`KismetStringLibrary.Conv_DoubleToString` _value_to_give)) true true (struct :`R` 0.191275 :`B` 1.0 :`A` 1.0) 0.0))
  (bind _success (message `/Game/Blueprints/Interfaces/IBP_Resources.Decrease Resource` (`self.CBP_Inventory`) "NewEnumerator1" (/ DeltaSeconds 100.0)))
  (`self.Turn on the Fire` _success)
  (`self.Update Widget` "NewEnumerator1"))

(event `self.Box.OnClicked`
  (params (TouchedComponent :type "PrimitiveComponent Object Reference") (ButtonPressed :type "Key Structure"))
  (bind (_color_current_kisel_r _color_current_kisel_g _color_current_kisel_b _color_current_kisel_a) (break `LinearColor` (`self.Color Current Kisel`)))
  ;[1 1 1] Если по объекту тыкнули мышкой, проверяем, близко ли персонаж игрока, если близко, то нужно принять от него ресурс
  (for _array_element (`PrimitiveComponent.GetOverlappingActors` (`self.Interact Box`) "/Game/Blueprints/Character/Character/BP_Character.BP_Character_C")
    (set `self.Array Element` _array_element)
    (if (== _array_element (`GameplayStatics.GetPlayerCharacter` 0))
      (message `/Game/Blueprints/Interfaces/IBP_QTE.Set Mouse Tag` (`self.Array Element`) (struct :`TagName` "Mouse Tags.Holding"))
      (bind _current_tag (message `/Game/Blueprints/Interfaces/IBP_Inventory.Get Current Tag` (`self.Array Element`)))
      (bind _resource (`self.Resource on switch` _current_tag))
      (bind _can_get_more (`/Game/Blueprints/Components/CBP_Inventory.Allready Max?` (`self.CBP_Inventory`) _resource))
      (if _can_get_more
        (bind (_type_of_resource_out _counter _have) (message `/Game/Blueprints/Interfaces/IBP_Resources.Get Resource from this one` (`self.Array Element`) "NewEnumerator0")) ; Начало рекурсивной цепочки сбора ресурса у персонажа игрока. \nЗдесь и только здесь не важно, как стоит входной ресурс.
        (if _have
          (message `/Game/Blueprints/Interfaces/IBP_Resources.Give Resource to this one` (`self.CBP_Inventory`) _type_of_resource_out _counter) ; Передаём ресурс в котёл
          (`self.Update Widget` _type_of_resource_out)
          (`self.Chose new color of Kisel`)
          (bind _value_to_give (`/Game/Blueprints/Components/CBP_Inventory.Get Value of Resource` (`self.CBP_Inventory`) "NewEnumerator0"))
          (bind _max_of_this_resource (`/Game/Blueprints/Components/CBP_Inventory.Get Max of Resource` (`self.CBP_Inventory`) "NewEnumerator0"))
          (`/Game/GUI/BPW_Cauldron_Widget.Set Cauldron Percent and Color` (`self.As BPW Cauldron Widget`) (/ _value_to_give _max_of_this_resource) (`KismetMathLibrary.MakeVector` _color_current_kisel_r _color_current_kisel_g _color_current_kisel_b) _color_current_kisel_a)
          (else
            (`KismetSystemLibrary.PrintString` "В котёл ничего не положили")))
        (else
          (`KismetSystemLibrary.PrintString` "В котле нет места для этого!"))))))

(event `self.Interact Box.OnComponentBeginOverlap`
  (params (OverlappedComponent :type "PrimitiveComponent Object Reference") (OtherActor :type "Actor Object Reference") (OtherComp :type "PrimitiveComponent Object Reference") (OtherBodyIndex :type Integer) (bFromSweep :type Boolean) (SweepResult :type "HitResult Structure (by ref)"))
  ;[1 1 1] Когда подошли к котлу, появляется виджет взаимодействия с котлом
  (if (== OtherActor (`GameplayStatics.GetPlayerCharacter` 0))
    (`Widget.SetVisibility` (`self.As BPW Cauldron Operations`) "Visible")
    (`Widget.SetVisibility` (`self.As BPW Cauldron State`) "SelfHitTestInvisible")))

(event `self.Interact Box.OnComponentEndOverlap`
  (params (OverlappedComponent :type "PrimitiveComponent Object Reference") (OtherActor :type "Actor Object Reference") (OtherComp :type "PrimitiveComponent Object Reference") (OtherBodyIndex :type Integer))
  ;[1 1 1] Когда отошли от котла, появляется виджет взаимодействия с котлом
  (if (== OtherActor (`GameplayStatics.GetPlayerCharacter` 0))
    (`Widget.SetVisibility` (`self.As BPW Cauldron Operations`) "Hidden")
    (`Widget.SetVisibility` (`self.As BPW Cauldron State`) "Hidden")))

(event `/Game/Blueprints/Interfaces/IBP_Inventory.Delete All Resources To Pigs`
  (message `/Game/Blueprints/Interfaces/IBP_Inventory.Delete All Resources To Pigs` (`self.CBP_Inventory`)))

(fn `Chose new color of Kisel`
  (bind _kisel_parametrs_berrieswater (break `/Game/Blueprints/Enviroment/Cauldron/ST_Kisel` (`self.Kisel Parametrs`)))
  (bind _color_and_opacity (`/Game/GUI/BPW_Cauldron_Widget.Get Cauldron Color` (`self.As BPW Cauldron Widget`)))
  (`self.Set Kisel Parametrs`)
  (set `self.Color Current Kisel` (make `LinearColor` (break `LinearColor` _color_and_opacity) (`KismetMathLibrary.MapRangeClamped` _kisel_parametrs_berrieswater 0.0 0.99 1.0 0.2) (`.B` (break `LinearColor` _color_and_opacity)) (`KismetMathLibrary.MapRangeClamped` _kisel_parametrs_berrieswater 0.0 0.99 0.5 1.0))))

(fn `Get Current Tag`
  (returns (`Current Tag` :type "GameplayTag Structure"))
  (return))

(fn `Get Inventory Gameplay Tag`
  (returns (`Inventory Tag` :type "GameplayTag Structure"))
  (return))

(fn `Get Kisel Parametrs`
  (returns (Kisel :type "/Game/Blueprints/Enviroment/Cauldron/ST_Kisel Structure"))
  (locals (`Berries/Water` :type "Float (double-precision)"))
  (bind _value_to_give (`/Game/Blueprints/Components/CBP_Inventory.Get Value of Resource` (`self.CBP_Inventory`) "NewEnumerator3"))
  (if (<= _value_to_give 0.0)
    (set `local.Berries/Water` 0.0)
    (else
      (bind _value_to_give_2 (`/Game/Blueprints/Components/CBP_Inventory.Get Value of Resource` (`self.CBP_Inventory`) "NewEnumerator0"))
      (if (> _value_to_give_2 0.0)
        (set `local.Berries/Water` (/ _value_to_give _value_to_give_2 0.01))
        (else
          (set `local.Berries/Water` 1.0)))))
  (bind _value_to_give_3 (`/Game/Blueprints/Components/CBP_Inventory.Get Value of Resource` (`self.CBP_Inventory`) "NewEnumerator1"))
  (return (make `/Game/Blueprints/Enviroment/Cauldron/ST_Kisel` (`local.Berries/Water`) _value_to_give_3)))

(fn `Get Mouse Tag`
  (returns (`Mouse Tag` :type "GameplayTag Structure"))
  (return))

(fn `Get ZOffset`
  (returns (`Get ZOffset` :type "Float (double-precision)"))
  (return 0.0))

(fn `Has Tag`
  (params (Tag :type "GameplayTag Structure"))
  (returns (`Has Tag` :type Boolean))
  (return false))

(fn `Resource on switch`
  (params (`Inventory tag of carrier` :type "GameplayTag Structure"))
  (returns (Resource :type "/Game/Blueprints/Enviroment/Enum_Resources Enum"))
  (locals (Resources :type "/Game/Blueprints/Enviroment/Enum_Resources Enum"))
  (`|SwitchGameplayTag` `Inventory tag of carrier`
    (:`Inventory Tags.Have Heavy Object.Berry Busket`
      (set `local.Resources` "NewEnumerator3"))
    (:`Inventory Tags.Have Heavy Object.Bucket`
      (set `local.Resources` "NewEnumerator0"))
    (:`Inventory Tags.Have Heavy Object.Wood`
      (set `local.Resources` "NewEnumerator1")))
  (return (`local.Resources`)))

(fn `Set Heavy Item`
  (params (Object :type "Actor Object Reference"))
  (returns (Success :type Boolean))
  (return false))

(fn `Set Kisel Parametrs`
  (locals (`Berries/Water` :type "Float (double-precision)" :default 1.0))
  (bind _value_to_give (`/Game/Blueprints/Components/CBP_Inventory.Get Value of Resource` (`self.CBP_Inventory`) "NewEnumerator3"))
  (if (<= _value_to_give 0.0)
    (set `local.Berries/Water` 0.0)
    (else
      (bind _value_to_give_2 (`/Game/Blueprints/Components/CBP_Inventory.Get Value of Resource` (`self.CBP_Inventory`) "NewEnumerator0"))
      (if (> _value_to_give_2 0.0)
        (set `local.Berries/Water` (/ _value_to_give _value_to_give_2 0.01))
        (else
          (set `local.Berries/Water` 0.0)))))
  (bind _value_to_give_3 (`/Game/Blueprints/Components/CBP_Inventory.Get Value of Resource` (`self.CBP_Inventory`) "NewEnumerator1"))
  (set `self.Kisel Parametrs` (make `/Game/Blueprints/Enviroment/Cauldron/ST_Kisel` (`local.Berries/Water`) _value_to_give_3)))

(fn `Update Widget`
  (params (NewParam :type "/Game/Blueprints/Enviroment/Enum_Resources Enum" :default "NewEnumerator0"))
  (locals (`BPW Cauldron State` :type "/Game/GUI/BPW_CauldronState Object Reference") (`This Resource Counter` :type "Float (double-precision)" :default 0.0) (`This Resource` :type "/Game/Blueprints/Enviroment/Enum_Resources Enum" :default "NewEnumerator0") (`Local Max` :type "Float (double-precision)" :default 0.0) (Percent :type "Float (double-precision)"))
  (set `local.This Resource` NewParam)
  (bind _value_to_give (`/Game/Blueprints/Components/CBP_Inventory.Get Value of Resource` (`self.CBP_Inventory`) (`local.This Resource`)))
  (set `local.This Resource Counter` _value_to_give)
  (bind _max_of_this_resource (`/Game/Blueprints/Components/CBP_Inventory.Get Max of Resource` (`self.CBP_Inventory`) (`local.This Resource`)))
  (bind _output_get (set `local.Local Max` _max_of_this_resource))
  (set `local.Percent` (/ (`local.This Resource Counter`) _output_get))
  (switch `/Game/Blueprints/Enviroment/Enum_Resources` (`local.This Resource`)
    (:`NewEnumerator0`
      (`/Game/GUI/BPW_CauldronState.Set Water Percent` (`self.As BPW Cauldron State`) (`local.Percent`)))
    (:`NewEnumerator1`
      (`/Game/GUI/BPW_CauldronState.Set Wood Percent` (`self.As BPW Cauldron State`) (`local.Percent`)))
    (:`NewEnumerator3`
      (`/Game/GUI/BPW_CauldronState.Set Berry Percent` (`self.As BPW Cauldron State`) (`local.Percent`)))))

(fn `UserConstructionScript`)