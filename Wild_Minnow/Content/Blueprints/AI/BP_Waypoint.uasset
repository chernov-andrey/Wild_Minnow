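; BP_Waypoint is an AI waypoint actor that one occupant at a time can reserve.
; TryReserve claims it only while IsOccupated is false, storing the occupant and reporting success.
; Release clears the reservation only when the requester matches the stored occupant.
; It has no active event or construction logic, so its state changes only through these calls.
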(fn `Release`
  (params (Requester :type "/Game/Blueprints/Character/BP_AI_Base Object Reference"))
  (returns (bReleased :type Boolean))
  (if (== Requester (`self.Occupant `))
    (set `self.IsOccupated` false)
    (set `self.Occupant ` null)
    (return true)
    (else
      (return false))))

(fn `Try Reserve`
  (params (`Occupant ` :type "/Game/Blueprints/Character/BP_AI_Base Object Reference"))
  (returns (`bSuccess ` :type Boolean) (OutputName :type "/Game/Blueprints/Character/BP_AI_Base Object Reference"))
  (if (not (`self.IsOccupated`))
    (set `self.IsOccupated` true)
    (bind _output_get (set `self.Occupant ` `Occupant `))
    (return true _output_get)
    (else
      (return false null))))

(fn `UserConstructionScript`)