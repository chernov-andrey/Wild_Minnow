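; BP_SpawnActor is an AI spawner that endlessly spawns actors at its billboard, passing each an ordered waypoint path.
; On BeginPlay it gathers all BP_Waypoint actors and sorts them by placing each at its OrderIndex.
; It spawns BP_AI and BP_AI2 first, then loops on a fixed delay.
; Looped spawns pick their class by cumulative-weight random roll over the SSpawn array, on a 0–100 scale.
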(event `Spawn`
  (bind _newlocalvar1 (`self.NewFunction`))
  (`|SpawnActorFromClass` _newlocalvar1 (`KismetMathLibrary.MakeTransform` (`SceneComponent.K2_GetComponentLocation` (`self.Billboard`))) "Undefined" "MultiplyWithRoot" null (`self.SortedWaypoints`) null)
  (`KismetSystemLibrary.Delay` 4.0)
  (`self.Spawn`))

(event `self.ReceiveBeginPlay`
  (bind _outactors (`GameplayStatics.GetAllActorsOfClass` "/Game/Blueprints/AI/BP_Waypoint.BP_Waypoint_C"))
  (bind _output_get (set `self.Unsortedwaypoints` _outactors))
  (bind _sorttedwaypoints (`self.SortWaypoints` _output_get))
  (set `self.SortedWaypoints` _sorttedwaypoints)
  (`self.FirstSpawn`))

(event `FirstSpawn`
  (`|SpawnActorFromClass` "/Game/Blueprints/Character/AI/BP_AI.BP_AI_C" (`KismetMathLibrary.MakeTransform` (`SceneComponent.K2_GetComponentLocation` (`self.Billboard`))) "Undefined" "MultiplyWithRoot" null (`self.SortedWaypoints`) null)
  (`KismetSystemLibrary.Delay` 4.0)
  (`|SpawnActorFromClass` "/Game/Blueprints/Character/AI2/BP_AI2.BP_AI2_C" (`KismetMathLibrary.MakeTransform` (`SceneComponent.K2_GetComponentLocation` (`self.Billboard`))) "Undefined" "MultiplyWithRoot" null (`self.SortedWaypoints`) null)
  (`KismetSystemLibrary.Delay` 4.0)
  (`self.Spawn`))

(fn `NewFunction`
  (returns (NewLocalVar1 :type "/Game/Blueprints/Character/BP_AI_Base Class Reference"))
  (locals (Road :type "Float (double-precision)") (Added :type "Float (double-precision)") (NewLocalVar :type "/Game/Blueprints/Character/BP_AI_Base Class Reference"))
  (set `local.Road` (`KismetMathLibrary.RandomFloatInRange` 0.0 100.0))
  (set `local.Added` 0.0)
  (for _array_element (`self.S_spawn`)
    (bind (_membervar_0 _membervar_1) (break `/Game/Blueprints/AI/S_Spawn` _array_element))
    (set `local.NewLocalVar` _membervar_0)
    (set `local.Added` (+ _membervar_1 (`local.Added`)))
    (if (< (`local.Road`) (`local.Added`))
      (break)))
  (return (`local.NewLocalVar`)))

(fn `SortWaypoints`
  (params (Waypoints :type "Array of /Game/Blueprints/AI/BP_Waypoint Object Reference"))
  (returns (SorttedWaypoints :type "Array of /Game/Blueprints/AI/BP_Waypoint Object Reference"))
  (`KismetArrayLibrary.Array_Clear` (`self.SortedWaypoints`))
  (for _array_element Waypoints
    (`KismetArrayLibrary.Array_Set` (`self.SortedWaypoints`) (`/Game/Blueprints/AI/BP_Waypoint.OrderIndex` _array_element) _array_element true))
  (return (`self.SortedWaypoints`)))

(fn `UserConstructionScript`)