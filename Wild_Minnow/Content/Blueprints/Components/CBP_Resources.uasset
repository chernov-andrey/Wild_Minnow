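; CBP_Resources is a resource component that describes one resource through ThisResource, a type and counter pair.
; Two near-duplicate getters return the type, and GetResourceFromThisOne reports type and counter with Have always true, ignoring the requested type and deducting nothing.
; DecreaseResource and GiveResourceToThisOne are placeholders that only return false.
; BeginPlay and Tick are empty, and a debug print is disconnected.
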(fn `Decrease Resource`
  (params (`Type of Resource` :type "/Game/Blueprints/Enviroment/Enum_Resources Enum" :default "NewEnumerator0") (Value :type "Float (double-precision)"))
  (returns (Success :type Boolean))
  (return false))

(fn `Get Resource from this one`
  (params (`Type of Resource in` :type "/Game/Blueprints/Enviroment/Enum_Resources Enum" :default "NewEnumerator0"))
  (returns (`Type of Resource out` :type "/Game/Blueprints/Enviroment/Enum_Resources Enum") (Counter :type "Float (double-precision)") (Have :type Boolean))
  (bind (_this_resource_resourcetype _this_resource_counter) (break `/Game/Blueprints/Structures/ST_Resources` (`self.This Resource`)))
  (return _this_resource_resourcetype _this_resource_counter true))

(fn `Get Type of Resorce`
  (returns (NewParam :type "/Game/Blueprints/Enviroment/Enum_Resources Enum"))
  (bind _this_resource_resourcetype (break `/Game/Blueprints/Structures/ST_Resources` (`self.This Resource`)))
  (return _this_resource_resourcetype))

(fn `Get Type of Resource`
  (returns (`Type of Resource` :type "/Game/Blueprints/Enviroment/Enum_Resources Enum"))
  (bind _this_resource_resourcetype (break `/Game/Blueprints/Structures/ST_Resources` (`self.This Resource`)))
  (return _this_resource_resourcetype))

(fn `Give Resource to this one`
  (params (`Type of Resource` :type "/Game/Blueprints/Enviroment/Enum_Resources Enum" :default "NewEnumerator0") (Counter :type "Float (double-precision)"))
  (returns (`Have to Give` :type Boolean))
  (return false))