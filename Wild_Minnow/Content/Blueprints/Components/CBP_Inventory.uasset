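; Inventory component that tracks an owner's resource amounts and a single carried heavy-item slot.
; Enum-keyed maps hold amounts, maximums and portion sizes; giving clamps to the maximum, taking yields one portion or the remainder.
; The heavy item's Empty tag follows filling and depletion, updating the owner's sprite; dropping detaches it ahead of the owner and clears its inventory tag.
; AllreadyMax returns true when below maximum, contrary to its name.
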(event `/Game/Blueprints/Interfaces/IBP_Inventory.Delete Heavy Item`
  ;[1 1 1] Убираем тяжелый предмет из рук
  (`self.Delete Heavy Item Helper`))

(event `/Game/Blueprints/Interfaces/IBP_Inventory.Delete All Resources To Pigs`
  ;[1 1 1] Очищаем все ресурсы отсюда
  (for _array_element (`self.Enum`)
    (if (`.ReturnValue` (`BlueprintMapLibrary.Map_Find` (`self.Resources of this Object`) _array_element))
      (`BlueprintMapLibrary.Map_Add` (`self.Resources of this Object`) _array_element)))
  (`KismetSystemLibrary.PrintString` "Ах, кончился кисель, как жаль"))

(fn `Allready Max?`
  (params (`Resource in` :type "/Game/Blueprints/Enviroment/Enum_Resources Enum" :default "NewEnumerator0"))
  (returns (`Can get more` :type Boolean))
  (bind _value_to_give (`self.Get Value of Resource` `Resource in`))
  (bind _less (`self.Less Than Max?` `Resource in` _value_to_give))
  (return _less))

(fn `Decrease Resource`
  (params (`Type of Resource` :type "/Game/Blueprints/Enviroment/Enum_Resources Enum" :default "NewEnumerator0") (Value :type "Float (double-precision)"))
  (returns (Success :type Boolean))
  (locals (`Local Type` :type "/Game/Blueprints/Enviroment/Enum_Resources Enum" :default "NewEnumerator0") (`Local Value` :type "Float (double-precision)" :default 0.0))
  (bind _have_this_resource (`self.Have to Give?` `Type of Resource`))
  (if _have_this_resource
    (bind _output_get (set `local.Local Type` `Type of Resource`))
    (bind _output_get_2 (set `local.Local Value` Value))
    (bind (_value _returnvalue) (`BlueprintMapLibrary.Map_Find` (`self.Resources of this Object`) _output_get))
    (if _returnvalue
      (`BlueprintMapLibrary.Map_Add` (`self.Resources of this Object`) (`local.Local Type`) (- _value _output_get_2))
      (return true)
      (else
        _)))
  (return false))

(fn `Delete Heavy Item Helper`
  (locals (`Local Rotator` :type "Rotator Structure" :default (struct)) (Scalar :type "Float (double-precision)" :default 100.0) (`Object Type` :type "Array of EObjectTypeQuery Enum"))
  (bind _owner (`self.Owner`))
  (bind (_returnvalue_x _returnvalue_y) (`KismetMathLibrary.BreakVector` (`SceneComponent.GetForwardVector` (`Actor.RootComponent` _owner))))
  (bind (_returnvalue_x_2 _returnvalue_y_2 _returnvalue_z) (`KismetMathLibrary.BreakVector` (+ (`Actor.K2_GetActorLocation` _owner) (* (`KismetMathLibrary.MakeVector` _returnvalue_x _returnvalue_y) (`local.Scalar`)))))
  (bind _rotator (`/Game/Blueprints/Character/Character/BP_Character.Get Rotator` _owner))
  (set `local.Local Rotator` _rotator)
  (message `/Game/Blueprints/Interfaces/IBP_Inventory.Get ZOffset` (`self.Heavy Item Slot`))
  (`Actor.K2_SetActorLocation` (`self.Heavy Item Slot`) (`KismetMathLibrary.MakeVector` _returnvalue_x_2 _returnvalue_y_2 (- _returnvalue_z 100.0)) false true)
  (`Actor.K2_DetachFromActor` (`self.Heavy Item Slot`) "KeepWorld" "KeepWorld" "KeepWorld")
  (bind _inventory_tag (message `/Game/Blueprints/Interfaces/IBP_Inventory.Get Inventory Gameplay Tag` (`self.Heavy Item Slot`)))
  (`/Game/Blueprints/Character/Character/BP_Character.Remove Inventory Tag` (`self.Owner`) _inventory_tag)
  (set `self.Heavy Item Slot` null))

(fn `Get Current Tag`
  (returns (`Current Tag` :type "GameplayTag Structure"))
  (return))

(fn `Get Heavy Item`
  (returns (`Heavy Item Slot` :type "Actor Object Reference"))
  (return (`self.Heavy Item Slot`)))

(fn `Get Inventory Gameplay Tag`
  (returns (`Inventory Tag` :type "GameplayTag Structure")))

(fn `Get Max of Resource`
  (params (`Type of resource` :type "/Game/Blueprints/Enviroment/Enum_Resources Enum" :default "NewEnumerator0"))
  (returns (`Max of this resource` :type "Float (double-precision)"))
  (bind (_value _returnvalue) (`BlueprintMapLibrary.Map_Find` (`self.Max Resources of this Object`) `Type of resource`))
  (if _returnvalue
    (return _value)
    (else
      (return 0.0))))

(fn `Get Portion of Resource`
  (params (`Type of Resource ` :type "/Game/Blueprints/Enviroment/Enum_Resources Enum" :default "NewEnumerator0"))
  (returns (`Value to give` :type "Float (double-precision)"))
  (locals (`I have this amount of resource` :type "Float (double-precision)") (`This Resource` :type "/Game/Blueprints/Enviroment/Enum_Resources Enum" :default "NewEnumerator0") (`Take this portion of resource` :type "Float (double-precision)"))
  (bind (_value _returnvalue) (`BlueprintMapLibrary.Map_Find` (`self.Resources of this Object`) (`local.This Resource`)))
  ;[1 1 1] Если у нас есть этот тип ресурса
  (bind _output_get (set `local.This Resource` `Type of Resource `))
  (bind (_value_2 _returnvalue_2) (`BlueprintMapLibrary.Map_Find` (`self.Dose of Resource to Give`) _output_get))
  (if _returnvalue_2
    (set `local.Take this portion of resource` _value_2)
    (if _returnvalue
      (set `local.I have this amount of resource` _value)
      ;[1 1 1] И у нас его меньше, чем мы хотим забрать, то отдаём всё
      (if (>= (`local.Take this portion of resource`) _value)
        (`BlueprintMapLibrary.Map_Add` (`self.Resources of this Object`) (`local.This Resource`))
        (bind _heavy_item_slot (`self.Get Heavy Item`))
        (message `/Game/Blueprints/Interfaces/IBP_Inventory.Add Tag` _heavy_item_slot (struct :`TagName` "Inventory Tags.Empty"))
        (`/Engine/EditorBlueprintResources/StandardMacros.IsValid` (`self.Owner`)
          (:`Is Valid`
            (`/Game/Blueprints/Character/Character/BP_Character.Change Sprite` (`self.Owner`) (struct :`TagName` "Inventory Tags.Empty")))
          (:`Is Not Valid`
            _))
        (return (`local.I have this amount of resource`))
        (else
          ;[1 1 1] Если у нас больше ресурсов, чем хотим забрать, то вычитаем, разницу в инвентарь, порцию выдаем на возврат
          (`BlueprintMapLibrary.Map_Add` (`self.Resources of this Object`) (`local.This Resource`) (- (`local.I have this amount of resource`) (`local.Take this portion of resource`)))
          (return (`local.Take this portion of resource`)))))))

(fn `Get Resource from this one`
  (params (`Type of Resource in` :type "/Game/Blueprints/Enviroment/Enum_Resources Enum" :default "NewEnumerator0"))
  (returns (`Type of Resource out` :type "/Game/Blueprints/Enviroment/Enum_Resources Enum") (Counter :type "Float (double-precision)") (Have :type Boolean))
  (locals (NewLocalVar :type "/Game/Blueprints/Enviroment/Enum_Resources Enum" :default "NewEnumerator0"))
  (bind (_value _returnvalue) (`BlueprintMapLibrary.Map_Find` (`self.Dose of Resource to Give`) `Type of Resource in`))
  (if _returnvalue
    (bind _value_to_give (`self.Get Portion of Resource` `Type of Resource in`))
    (return `Type of Resource in` _value_to_give _returnvalue)))

(fn `Get Type of Resorce`
  (returns (NewParam :type "/Game/Blueprints/Enviroment/Enum_Resources Enum"))
  (return "NewEnumerator0"))

(fn `Get Value of Resource`
  (params (`Type of Resource` :type "/Game/Blueprints/Enviroment/Enum_Resources Enum" :default "NewEnumerator0"))
  (returns (`Value to give` :type "Float (double-precision)"))
  (locals (`I have this amount of resource` :type "Float (double-precision)"))
  (bind (_value _returnvalue) (`BlueprintMapLibrary.Map_Find` (`self.Resources of this Object`) `Type of Resource`))
  ;[1 1 1] Сообщаем, сколько у нас этого ресурса
  (if _returnvalue
    (bind _output_get (set `local.I have this amount of resource` _value))
    (return _output_get)))

(fn `Get ZOffset`
  (returns (`Get ZOffset` :type "Float (double-precision)"))
  (return 0.0))

(fn `Give Resource to this one`
  (params (`Type of Resource` :type "/Game/Blueprints/Enviroment/Enum_Resources Enum" :default "NewEnumerator0") (Counter :type "Float (double-precision)"))
  (returns (`Have to Give` :type Boolean))
  (bind (_value _returnvalue) (`BlueprintMapLibrary.Map_Find` (`self.Resources of this Object`) (`self.Type Of Resource`)))
  (bind _returnvalue_2 (+ _value (`self.Counter`)))
  ;[1 1 1] Собрать этот ресурс в сооветствующий слот
  (set `self.Type Of Resource` `Type of Resource`)
  (set `self.Counter` Counter)
  (if _returnvalue
    (bind _less (`self.Less Than Max?` (`self.Type Of Resource`) _value))
    (if _less
      (bind _less_2 (`self.More Than Max?` (`self.Type Of Resource`) _returnvalue_2))
      (if _less_2
        (`self.Set Max` (`self.Type Of Resource`))
        (`KismetSystemLibrary.PrintString` "Место кончилось!")
        (return true)
        (else
          (bind _heavy_item_slot (`self.Get Heavy Item`))
          (bind _has_tag (message `/Game/Blueprints/Interfaces/IBP_Inventory.Has Tag` _heavy_item_slot (struct :`TagName` "Inventory Tags.Empty")))
          (if _has_tag
            (message `/Game/Blueprints/Interfaces/IBP_Inventory.Remove Tag` _heavy_item_slot (struct :`TagName` "Inventory Tags.Empty"))
            (`/Engine/EditorBlueprintResources/StandardMacros.IsValid` (`self.Owner`)
              (:`Is Valid`
                (`/Game/Blueprints/Character/Character/BP_Character.Change Sprite` :`self` (`self.Owner`)))
              (:`Is Not Valid`
                _)))
          (`BlueprintMapLibrary.Map_Add` (`self.Resources of this Object`) (`self.Type Of Resource`) _returnvalue_2)
          (`KismetSystemLibrary.PrintString` "Место еще есть!")
          (return true))))))

(fn `Has Tag`
  (params (Tag :type "GameplayTag Structure"))
  (returns (`Has Tag` :type Boolean))
  (return false))

(fn `Have to Give?`
  (params (`Type of Resource` :type "/Game/Blueprints/Enviroment/Enum_Resources Enum" :default "NewEnumerator0"))
  (returns (`Have this Resource` :type Boolean))
  (bind (_value _returnvalue) (`BlueprintMapLibrary.Map_Find` (`self.Resources of this Object`) `Type of Resource`))
  (if _returnvalue
    (return (> _value 0.0))
    (else
      (return false))))

(fn `Less Than Max?`
  (params (`Type of Resource` :type "/Game/Blueprints/Enviroment/Enum_Resources Enum" :default "NewEnumerator0") (Value :type "Float (double-precision)"))
  (returns (Less :type Boolean))
  (bind _max_of_this_resource (`self.Get Max of Resource` `Type of Resource`))
  (return (< Value _max_of_this_resource)))

(fn `More Than Max?`
  (params (`Type of Resource` :type "/Game/Blueprints/Enviroment/Enum_Resources Enum" :default "NewEnumerator0") (Value :type "Float (double-precision)"))
  (returns (Less :type Boolean))
  (bind _max_of_this_resource (`self.Get Max of Resource` `Type of Resource`))
  (return (>= Value _max_of_this_resource)))

(fn `Set Heavy Item`
  (params (Object :type "Actor Object Reference"))
  (returns (Success :type Boolean))
  ;[1 1 1] Помещаем тяжелый предмет в руки. Если слот уже занят другим объектом, то возвращаем неудачу, предмет нужно оставить
  (`/Engine/EditorBlueprintResources/StandardMacros.IsValid` (`self.Heavy Item Slot`)
    (:`Is Valid`
      (return false))
    (:`Is Not Valid`
      (bind _output_get (set `self.Heavy Item Slot` Object))
      (bind _inventory_tag (message `/Game/Blueprints/Interfaces/IBP_Inventory.Get Inventory Gameplay Tag` _output_get))
      (`/Game/Blueprints/Character/Character/BP_Character.Set Inventory Tag` (`self.Owner`) _inventory_tag)
      (return true))))

(fn `Set Max`
  (params (`Type of Resource` :type "/Game/Blueprints/Enviroment/Enum_Resources Enum" :default "NewEnumerator0"))
  (bind (_value _returnvalue) (`BlueprintMapLibrary.Map_Find` (`self.Max Resources of this Object`) `Type of Resource`))
  (if (and (`.ReturnValue` (`BlueprintMapLibrary.Map_Find` (`self.Resources of this Object`) `Type of Resource`)) _returnvalue)
    (`BlueprintMapLibrary.Map_Add` (`self.Resources of this Object`) `Type of Resource` _value)))

(fn `Set Owner`
  (params (Owner :type "/Game/Blueprints/Character/Character/BP_Character Object Reference"))
  (set `self.Owner` Owner))