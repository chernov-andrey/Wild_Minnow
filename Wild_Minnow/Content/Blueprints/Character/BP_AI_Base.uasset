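; Base AI pawn that queues along a waypoint array and destroys itself after the last one.
; MoveAi reserves a waypoint before walking to it; ForAiBreach holds the current one until the next is free, with both polling on short delays.
; At WaitAtIndex it stops until NextMove releases the waypoint and resumes movement.
; A sphere overlap tracks whether BP_Character is in range.
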(event `ForAiBreach`
  (if (`/Game/Blueprints/AI/BP_Waypoint.IsOccupated` (`self.NextReserverdWaypoint`))
    (`KismetSystemLibrary.Delay` 0.1)
    (`self.ForAiBreach`)
    (else
      (`/Game/Blueprints/AI/BP_Waypoint.Release` (`self.CurrentReservedWaypoint`) self)
      (`self.MoveAi`))))

(event `MoveAi`
  (bind _bsuccess_ (`/Game/Blueprints/AI/BP_Waypoint.Try Reserve` (`|GetArrayItem` (`self.Waypoints`) (`self.CurrentWaypoint`)) self))
  (if _bsuccess_
    (set `self.CurrentReservedWaypoint` (`|GetArrayItem` (`self.Waypoints`) (`self.CurrentWaypoint`)))
    (set `self.NextReserverdWaypoint` (`|GetArrayItem` (`self.Waypoints`) (+ (`self.CurrentWaypoint`) 1)))
    (`|AIMoveTo` self (0.0 0.0 0.0) (`|GetArrayItem` (`self.Waypoints`) (`self.CurrentWaypoint`))
      (:`OnSuccess`
        (`/Engine/EditorBlueprintResources/StandardMacros.IncrementInt` (`self.CurrentWaypoint`)
          (:`  `
            (if (== (`self.CurrentWaypoint`) (`self.WaitAtIndex`))
              (`KismetSystemLibrary.PrintString` "Жду кнопки взаимодействия , как меня вызовут")
              (elif (>= (`self.CurrentWaypoint`) (`KismetArrayLibrary.Array_Length` (`self.Waypoints`)))
                (`/Game/Blueprints/AI/BP_Waypoint.Release` (`self.CurrentReservedWaypoint`) self)
                (`self.K2_DestroyActor`)
                (else
                  (`KismetSystemLibrary.Delay` (`self.DelayWaypointNext`))
                  (`self.ForAiBreach`))))))))
    (else
      (`KismetSystemLibrary.Delay` 0.1)
      (`self.MoveAi`))))

(event `NextMove`
  (if (== (`self.CurrentWaypoint`) (`self.WaitAtIndex`))
    (`KismetSystemLibrary.PrintString` "Да, я в точке остановки и пойду в следующую")
    (`/Game/Blueprints/AI/BP_Waypoint.Release` (`self.CurrentReservedWaypoint`) self)
    (`self.MoveAi`)
    (else
      (`KismetSystemLibrary.PrintString` "я еще не  в последней точке"))))

(event `self.Sphere.OnComponentBeginOverlap`
  (params (OverlappedComponent :type "PrimitiveComponent Object Reference") (OtherActor :type "Actor Object Reference") (OtherComp :type "PrimitiveComponent Object Reference") (OtherBodyIndex :type Integer) (bFromSweep :type Boolean) (SweepResult :type "HitResult Structure (by ref)"))
  (cast `/Game/Blueprints/Character/Character/BP_Character` OtherActor)
  (set `self.PlayerInRange` true))

(event `self.Sphere.OnComponentEndOverlap`
  (params (OverlappedComponent :type "PrimitiveComponent Object Reference") (OtherActor :type "Actor Object Reference") (OtherComp :type "PrimitiveComponent Object Reference") (OtherBodyIndex :type Integer))
  (cast `/Game/Blueprints/Character/Character/BP_Character` OtherActor)
  (set `self.PlayerInRange` false))

(event `self.ReceiveBeginPlay`
  (`parent.ReceiveBeginPlay`)
  (`self.SpawnDefaultController`)
  (`self.MoveAi`))

(fn `UserConstructionScript`
  (`parent.UserConstructionScript`))