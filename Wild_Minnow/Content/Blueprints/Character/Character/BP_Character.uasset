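; Player character Blueprint with Enhanced Input movement, resource gathering and carrying of heavy items such as buckets, wood and berry baskets.
; Resource and item calls forward to CBPInventory, with inventory gameplay tags deciding which resource GetResource hands over and wood being destroyed afterwards.
; Cursor tags gate a left-button hold that shows a delayed progress widget following the mouse.
; Debug keys test dropping the heavy item and a QTE progress bar.
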(event Input|EnhancedActionEvents|EnhancedInputActionIA_Move
  (params (ActionValue :type Vector%202D%20Structure) (ElapsedSeconds :type Float%20%28double-precision%29) (TriggeredSeconds :type Float%20%28double-precision%29) (InputAction :type Input%20Action%20Object%20Reference :default "/Game/GameSettings/Input/Actions/IA_Move.IA_Move"))
  (bind (_x _y) (Math|Vector2D|BreakVector2D ActionValue))
  ;[1 1 1] Передвижение
  (Pawn|Input|AddMovementInput "1.000000,0.000000,0.000000" _x false)
  (Pawn|Input|AddMovementInput "0.000000,1.000000,0.000000" _y false))

(event Input|EnhancedActionEvents|EnhancedInputActionIA_LMB
  (params (ActionValue :type Boolean) (ElapsedSeconds :type Float%20%28double-precision%29) (TriggeredSeconds :type Float%20%28double-precision%29) (InputAction :type Input%20Action%20Object%20Reference :default "/Game/GameSettings/Input/Actions/IA_LMB.IA_LMB"))
  ;[1 1 1] Реализация удержания левой кнопки мыши
  (:Ongoing
    (if (GameplayTags|HasTag (Variables|Default|GetCursor%20Tags) "(TagName=\"Mouse Tags.Holding\")" true)
      ;;[1 1 1] Чтобы курсор отображался не сразу, часть 1
      (bind _output_get (Variables|Default|SetOngoing ElapsedSeconds))
      (if (> _output_get 1.0)
        (Default|SetCursorHolding (Variables|Default|GetAs%20BPW%20Cursor%20Widget%20Holding))
        (Class|PlayerController|SetMouseCursorWidget (Game|GetPlayerController 0) "Hand" (Variables|Default|GetAs%20BPW%20Cursor%20Widget%20Holding))
        (Default|SetProgressPercent (Variables|Default|GetAs%20BPW%20Cursor%20Widget%20Holding) (/ (- (Variables|Default|GetOngoing) 1.0) 2.0)))))
  (:Canceled
    (Default|SetCursorDefault (Variables|Default|GetAs%20BPW%20Cursor%20Widget%20Holding) :!label _label)
    (CallFunction|RemoveMouseTag "(TagName=\"Mouse Tags.Holding\")"))
  (:Completed
    (goto _label)))

(event EventBeginPlay
  ;[1 1 1] Инициализация движения, задания управления
  (|CallParentFunction)
  (bind _asplayer_controller (Utilities|Casting|CastToPlayerController (Pawn|GetController)))
  (Input|AddMappingContext (PlayerController|LocalPlayerSubsystems|GetEnhancedInputLocalPlayerSubsystem _asplayer_controller) "/Game/GameSettings/Input/IMC_Game.IMC_Game" 0 "(bIgnoreAllPressedKeysUntilRelease=True,bForceImmediately=False,bNotifyUserSettings=False)")
  ;[1 1 1] Сообщаем инвентарю владельца (Себя)
  (Default|SetOwner (Variables|Default|GetCBP_Inventory) self)
  ;[1 1 1] Тест QTE
  (bind _asbpw_test (Utilities|Casting|CastToBPW_Test (UserInterface|GetWidget (Variables|Default|GetTest%20Widget))))
  (Variables|Default|SetAs%20BPW%20Test _asbpw_test)
  ;[1 1 1] Задаём виджет курсора
  (bind _returnvalue (UserInterface|CreateWidget "/Game/GUI/BPW_CursorWidgetHolding.BPW_CursorWidgetHolding_C" (Game|GetPlayerController 0)))
  (bind _output_get (Variables|Default|SetAs%20BPW%20Cursor%20Widget%20Holding _returnvalue))
  (UserInterface|Viewport|AddtoViewport _output_get 0))

(event EventGiveResource
  (params (Type%20of%20Resource :type Enum_Resources%20Enum :default "NewEnumerator0") (Counter :type Float%20%28double-precision%29))
  ;[1 1 1] Получение ресурсов и передача их в инвентарь. Думал сделать так, что если в руках ведро, то ресурс получает ведро, а не персонаж, но с точки зрения кода вообще всё равно пока что
  (Variables|Default|SetCounter Counter)
  (switch Utilities|FlowControl|Switch|SwitchonEnum_Resources Type%20of%20Resource
    (:NewEnumerator0
      _)
    (:NewEnumerator1
      _)
    (:NewEnumerator2
      _)
    (:NewEnumerator3
      _))
  (Default|GiveResource (Variables|Default|GetCBP_Inventory) Type%20of%20Resource (Variables|Default|GetCounter)))

(event EventTick
  (params (DeltaSeconds :type Float%20%28single-precision%29))
  ;[1 1 1] Перемещаем виджет-курсор
  (bind _returnvalue (Class|WidgetLayoutLibrary|GetMousePositiononViewport))
  (Class|UserWidget|SetPositioninViewport (Variables|Default|GetAs%20BPW%20Cursor%20Widget%20Holding) _returnvalue false))

(event EventSetMouseTag
  (params (Mouse%20Tag :type Gameplay%20Tag%20Structure))
  (GameplayTags|AddGameplayTag (Variables|Default|GetCursor%20Tags) Mouse%20Tag :!class /Script/GameplayTags.BlueprintGameplayTagLibrary))

(event EventRemoveMouseTag
  (params (Mouse%20Tag :type Gameplay%20Tag%20Structure))
  (GameplayTags|RemoveGameplayTag (Variables|Default|GetCursor%20Tags) Mouse%20Tag :!class /Script/GameplayTags.BlueprintGameplayTagLibrary))

(event Input|MouseEvents|DebugKeyRightMouseButton
  (params (Key :type Key%20Structure :default "None") (ActionValue :type Input%20Action%20Value%20Structure))
  ;[1 1 1] Тест, хватания определенных предметов на ЛКМ, ставятся на ПКМ, но без проверки что там
  (:Pressed
    (if (GameplayTags|HasTag (Variables|Default|GetInventory%20Tags) "(TagName=\"Inventory Tags.Have Heavy Object\")")
      (Default|DeleteHeavyItem (Variables|Default|GetCBP_Inventory))
      (Development|PrintString "Бросил предмет")
      (else
        (Development|PrintString "У меня ничего нет")))))

(event Input|KeyboardEvents|DebugKeyF
  (params (Key :type Key%20Structure :default "None") (ActionValue :type Input%20Action%20Value%20Structure))
  ;[1 1 1] Тест QTE на усилие, работает, доделать
  (:Pressed
    (bind _output_get (Variables|Default|SetTest (+ (Variables|Default|GetTest) 1e+01)))
    (Class|IBPQTE|SetProgressPercent(Message) (Variables|Default|GetAs%20BPW%20Test) (/ _output_get (Variables|Default|GetTest%20Max)))))

(fn ConstructionScript
  (|CallParentFunction))

(fn SetInventoryTag
  (params (Tag :type Gameplay%20Tag%20Structure))
  (GameplayTags|AddGameplayTag (Variables|Default|GetInventory%20Tags) Tag :!class /Script/GameplayTags.BlueprintGameplayTagLibrary))

(fn GetRotator
  (return (Class|CharacterMovementComponent|GetLastUpdateRotation (Variables|Character|GetCharacterMovement))))

(fn RemoveInventoryTag
  (params (Inventory%20Tag :type Gameplay%20Tag%20Structure))
  (GameplayTags|RemoveGameplayTag (Variables|Default|GetInventory%20Tags) Inventory%20Tag :!class /Script/GameplayTags.BlueprintGameplayTagLibrary))

(fn GetWidgetComponent
  (return (Variables|Default|GetTest%20Widget)))

(fn HasInventoryTag
  (params (Inventory%20Tag :type Gameplay%20Tag%20Structure))
  (return (GameplayTags|HasTag (Variables|Default|GetInventory%20Tags) Inventory%20Tag)))

(fn DecreaseResource
  (params (Type%20of%20Resource :type Enum_Resources%20Enum :default "NewEnumerator0") (Value :type Float%20%28double-precision%29))
  (return false))

(fn GetInventoryGameplayTag
  (return ""))

(fn GetMouseTag
  (return ""))

(fn GetResource
  (params (Type%20of%20Resource%20in :type Enum_Resources%20Enum :default "NewEnumerator0"))
  (|SwitchGameplayTagContainer (Variables|Default|GetInventory%20Tags)
    (:%28GameplayTags=%28%28TagName="Inventory%20Tags.Have%20Heavy%20Object.Bucket"%29%29%29
      (LocalVariables|SetNewLocalVar "NewEnumerator0"))
    (:%28GameplayTags=%28%28TagName="Inventory%20Tags.Have%20Heavy%20Object.Wood"%29%29%29
      (LocalVariables|SetNewLocalVar "NewEnumerator1"))
    (:%28GameplayTags=%28%28TagName="Inventory%20Tags.Have%20Heavy%20Object.Berry%20Busket"%29%29%29
      (LocalVariables|SetNewLocalVar "NewEnumerator3")))
  (bind _have_this_resource (Default|HavetoGive? (Variables|Default|GetCBP_Inventory) (LocalVariables|GetNewLocalVar)))
  (if _have_this_resource
    (bind (_type_of_resource_out _counter) (Default|GetResource (Variables|Default|GetCBP_Inventory) (LocalVariables|GetNewLocalVar)))
    (switch Utilities|FlowControl|Switch|SwitchonEnum_Resources _type_of_resource_out
      (:NewEnumerator0
        _)
      (:NewEnumerator1
        (bind _heavy_item_slot (Default|GetHeavyItem (Variables|Default|GetCBP_Inventory)))
        (LocalVariables|SetHeavy%20Item%20Ref _heavy_item_slot)
        (Default|DeleteHeavyItem (Variables|Default|GetCBP_Inventory))
        (Class|IBPResources|DestroyThisResourceObject(Message) (LocalVariables|GetHeavy%20Item%20Ref)))
      (:NewEnumerator2
        _)
      (:NewEnumerator3
        _))
    (return _type_of_resource_out _counter)
    (else
      (Development|PrintString (Utilities|String|Append "У меня нет этого ресурса: " (Utilities|String|EnumtoString (LocalVariables|GetNewLocalVar)))))))

(fn GetTypeOfResorce
  (return "NewEnumerator0"))

(fn SetHeavyItem
  (params (Object :type Actor%20Object%20Reference))
  (bind _success (Class|IBPInventory|SetHeavyItem(Message) (Variables|Default|GetCBP_Inventory) Object))
  (return _success))