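; Player character that moves on X/Y with a +Y boundary, carries one BP_Equip_UPDATE item and interacts with nearby actors.
; Attempt_Interact attaches the nearest equip when empty-handed, otherwise messages the nearest IBP_Interaction actor, both found by sphere overlap.
; RMB drops the held item at a +Y offset without checking the destination, toggling its sprite collision back on.
; Helper functions cover held-item checks, proximity tests and harvesting through the held item.
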(event `self.ReceiveBeginPlay`
  (`parent.ReceiveBeginPlay`)
  (bind _asbp_player_controller (cast `/Game/GameSettings/BP_PlayerController` (`self.GetController`)))
  (set `self.As BP Player Controller` _asbp_player_controller))

(event `EnhancedInput|/Game/GameSettings/Input/Actions/IA_Move`
  (params (ActionValue :type "Vector2D Structure") (ElapsedSeconds :type "Float (double-precision)") (TriggeredSeconds :type "Float (double-precision)") (InputAction :type "InputAction Object Reference" :default "/Game/GameSettings/Input/Actions/IA_Move.IA_Move"))
  (bind (_returnvalue_x _returnvalue_y) (`KismetMathLibrary.BreakVector` (`self.K2_GetActorLocation`)))
  (bind (_x _y) (`KismetMathLibrary.BreakVector2D` ActionValue))
  ;[0.3971 1 0.03355] Передвижение
  (:`Triggered`
    (`self.AddMovementInput` (1.0 0.0 0.0) _x)
    (if (> _y 0.0)
      (if (< _returnvalue_y -980.0)
        (`self.AddMovementInput` (0.0 1.0 0.0) _y :!label _label))
      (else
        (goto _label)))))

(event `EnhancedInput|/Game/GameSettings/Input/Actions/IA_RMB`
  (params (ActionValue :type Boolean) (ElapsedSeconds :type "Float (double-precision)") (TriggeredSeconds :type "Float (double-precision)") (InputAction :type "InputAction Object Reference" :default "/Game/GameSettings/Input/Actions/IA_RMB.IA_RMB"))
  (bind _inhand (`self.InHand`))
  (bind (_returnvalue_x _returnvalue_y) (`KismetMathLibrary.BreakVector` (`self.K2_GetActorLocation` _inhand)))
  ;[1 1 1] Тест, хватания определенных предметов на ЛКМ, ставятся на ПКМ, но без проверки что там
  (:`Triggered`
    (bind _isempty (`self.Is_Empty_Hand`))
    (if (not _isempty)
      (`self.K2_DetachFromActor` _inhand "KeepWorld" "KeepWorld" "KeepRelative")
      (`self.K2_SetActorLocation` _inhand (`KismetMathLibrary.MakeVector` _returnvalue_x (+ _returnvalue_y 300.0)) false false)
      (`PrimitiveComponent.SetCollisionEnabled` (`/Game/Test/BP_Equip_UPDATE.PaperSprite` _inhand) "QueryAndPhysics")
      (set `self.InHand` null))))

(event `Attempt_Interact`
  (bind _isempty (`self.Is_Empty_Hand`))
  (if _isempty
    (`self.Try_Pickup_Equip`)
    (else
      (`self.Try_Interact_with_Nearest_Actor`))))

(event `Try_Interact_with_Nearest_Actor`
  (bind _nearestactor (`self.Get Nearest Actor With Interface IBP Interact`))
  (message `/Game/Blueprints/Interfaces/IBP_Interaction.Try_interact` _nearestactor))

(event `/Game/Blueprints/Interfaces/IBP_Interaction.Try_Pickup_Equip`
  (bind (_nearestactor _result) (`self.Get Nearest Actors Of Class by Interface` "/Game/Test/BP_Equip_UPDATE.BP_Equip_UPDATE_C"))
  (if _result
    (`self.Pickup_Equip` _nearestactor)))

(fn `Get Nearest Actor With Interface IBP Interact`
  (returns (NearestActor :type "Actor Object Reference") (Result :type Boolean))
  (locals (Ators_with_Interface :type "Array of Actor Object Reference") (Nearest_Actor :type "Actor Object Reference") (MinDistance :type "Float (double-precision)"))
  (bind _ators_with_interface (`local.Ators_with_Interface`))
  (bind _output (`|GetArrayItem` _ators_with_interface))
  (bind (_outactors _returnvalue) (`KismetSystemLibrary.SphereOverlapActors` (`self.K2_GetActorLocation`) 200.0 (`|MakeArray` "ObjectTypeQuery1" "ObjectTypeQuery2" "ObjectTypeQuery3" "ObjectTypeQuery4" "ObjectTypeQuery5" "ObjectTypeQuery6" :!type "EObjectTypeQuery Enum") "/Script/Engine.Actor" (`|MakeArray` self :!type "Actor Object Reference")))
  (if _returnvalue
    (for _array_element _outactors
      (if (`KismetSystemLibrary.DoesImplementInterface` _array_element "/Game/Blueprints/Interfaces/IBP_Interaction.IBP_Interaction_C")
        (`KismetArrayLibrary.Array_Add` (`local.Ators_with_Interface`) _array_element)))
    (if (`KismetArrayLibrary.Array_IsEmpty` (`local.Ators_with_Interface`))
      (return null false)
      (elif (== (`KismetArrayLibrary.Array_Length` _ators_with_interface) 1)
        (return _output true)
        (else
          (set `local.Nearest_Actor` _output)
          (set `local.MinDistance` (`KismetMathLibrary.Vector_Distance` (`self.K2_GetActorLocation` (`local.Nearest_Actor`)) (`self.K2_GetActorLocation`)))
          (for _array_element_2 _ators_with_interface
            (bind _returnvalue_2 (`KismetMathLibrary.Vector_Distance` (`self.K2_GetActorLocation` _array_element_2) (`self.K2_GetActorLocation`)))
            (if (< _returnvalue_2 (`local.MinDistance`))
              (set `local.MinDistance` _returnvalue_2)
              (set `local.Nearest_Actor` _array_element_2)))
          (return (`local.Nearest_Actor`) true))))
    (else
      (return null false))))

(fn `Get Nearest Actors Of Class by Interface`
  (params (ClassActors :type "Object Class Reference"))
  (returns (NearestActor :type "Actor Object Reference") (Result :type Boolean))
  (locals (MinDistance :type "Float (double-precision)") (Nearest_Actor :type "Actor Object Reference"))
  (bind (_outactors _returnvalue) (`KismetSystemLibrary.SphereOverlapActors` (`self.K2_GetActorLocation`) 200.0 (`|MakeArray` "ObjectTypeQuery1" "ObjectTypeQuery2" "ObjectTypeQuery3" "ObjectTypeQuery4" "ObjectTypeQuery5" "ObjectTypeQuery6" :!type "EObjectTypeQuery Enum") ClassActors))
  (if _returnvalue
    (if (== (`KismetArrayLibrary.Array_Length` _outactors) 1)
      (bind _output (`|GetArrayItem` _outactors))
      (return _output true)
      (else
        (set `local.Nearest_Actor` _output)
        (set `local.MinDistance` (`KismetMathLibrary.Vector_Distance` (`self.K2_GetActorLocation` (`local.Nearest_Actor`)) (`self.K2_GetActorLocation`)))
        (for _array_element _outactors
          (bind _returnvalue_2 (`KismetMathLibrary.Vector_Distance` (`self.K2_GetActorLocation` _array_element) (`self.K2_GetActorLocation`)))
          (if (< _returnvalue_2 (`local.MinDistance`))
            (set `local.MinDistance` _returnvalue_2)
            (set `local.Nearest_Actor` _array_element)))
        (return (`local.Nearest_Actor`) true)))
    (else
      (return null false))))

(fn `Harvast`
  (returns (Success :type Boolean))
  (bind _there_is_place (`/Game/Test/BP_Equip_UPDATE.IsTherePlace` (`self.InHand`)))
  (if _there_is_place
    (`/Game/Test/BP_Equip_UPDATE.Give_item` (`self.InHand`))
    (return true)
    (else
      (return false))))

(fn `Is_Empty_Hand`
  (returns (IsEmpty :type Boolean))
  (return (== (`self.InHand`) null)))

(fn `IsNearby`
  (params (Actor :type "Actor Object Reference") (Distance_override :type "Float (double-precision)"))
  (returns (bNearby :type Boolean))
  (return (> (`KismetMathLibrary.SelectFloat` Distance_override (`self.Distance_Interact`) (> Distance_override 0.0)) (`KismetMathLibrary.Vector_Distance` (`self.K2_GetActorLocation` Actor) (`self.K2_GetActorLocation`)))))

(fn `IsThisEquiped_in_Hand`
  (params (Equip :type "/Game/Test/BP_Equip_UPDATE Object Reference"))
  (returns (InHand :type Boolean))
  (return (== Equip (`self.InHand`))))

(fn `Pickup_Equip`
  (params (EquipActor :type "Actor Object Reference"))
  (bind _asbp_equip_update (cast `/Game/Test/BP_Equip_UPDATE` EquipActor))
  (bind _output_get (set `self.InHand` _asbp_equip_update))
  (`PrimitiveComponent.SetCollisionEnabled` (`/Game/Test/BP_Equip_UPDATE.PaperSprite` _output_get) "NoCollision")
  (`self.K2_AttachToActor` _output_get self "soket" "SnapToTarget" "KeepWorld" "KeepWorld" true)
  (`self.K2_SetActorRelativeLocation` _output_get (-200.0 0.0 50.0) false false)
  (return))

(fn `UserConstructionScript`
  (`parent.UserConstructionScript`))