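; BP_AI is an AI-controlled pawn that patrols a looping route of waypoints.
; Shortly after BeginPlay, MoveAI runs AI MoveTo toward the current entry in the Waypoints array.
; On success it advances the index, wrapping to zero at the end, waits DelayWaypointNext, then calls itself again.
; A failed move has no handler, so the patrol stops there.
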(event `self.ReceiveBeginPlay`
  (`parent.ReceiveBeginPlay`)
  (`KismetSystemLibrary.Delay` 0.2)
  (`self.MoveAI`))

(event `MoveAI`
  (`|AIMoveTo` self (0.0 0.0 0.0) (`|GetArrayItem` (`self.Waypoints`) (`self.CurrentWaypoint`))
    (:`OnSuccess`
      (`/Engine/EditorBlueprintResources/StandardMacros.IncrementInt` (`self.CurrentWaypoint`)
        (:`  `
          (if (>= (`self.CurrentWaypoint`) (`KismetArrayLibrary.Array_Length` (`self.Waypoints`)))
            (set `self.CurrentWaypoint` 0))
          (`KismetSystemLibrary.Delay` (`self.DelayWaypointNext`))
          (`self.MoveAI`))))))

(fn `UserConstructionScript`
  (`parent.UserConstructionScript`))