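; BP_Equip_UPDATE is a test equipment container that holds a count of items up to a capacity.
; The construction script sets its PaperSprite from the Type enum (Water, Wood, RedBerry, BlueBerry), with no sprite assigned for RedBerry.
; IsTherePlace reports whether Content is below Capacity, and GiveItem increments Content without checking that limit itself.
; The event graph has no logic.
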(event `self.ReceiveTick`
  (params (DeltaSeconds :type "Float (single-precision)")))

(fn `Give_item`
  (`/Engine/EditorBlueprintResources/StandardMacros.IncrementInt` (`self.Content`)))

(fn `IsTherePlace`
  (returns (`There is place` :type Boolean))
  (return (< (`self.Content`) (`self.Capacity`))))

(fn `UserConstructionScript`
  (`PaperSpriteComponent.SetSprite` (`self.PaperSprite`) (select `/Game/Blueprints/Enviroment/Enum_Resources` (`self.Type`) :`NewEnumerator0` "/Game/Art/PaperAssets/Enviroment/Bucket/Bucket_Empty_Sprite.Bucket_Empty_Sprite" :`NewEnumerator1` "/Game/Art/PaperAssets/Enviroment/Wood/Wood_Sprite_0.Wood_Sprite_0" :`NewEnumerator3` "/Game/Art/PaperAssets/Enviroment/Berry_Buscket/Berry_Buscket_1_Sprite.Berry_Buscket_1_Sprite" :!type "PaperSprite Object Reference")))